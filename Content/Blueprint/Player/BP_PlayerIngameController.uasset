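; In-game player controller for picking up and placing team 0 units on board squares while their battlefield's battle is off.
; Each tick a cursor trace and small sphere trace find the focused square, highlight its unit and glide any held unit toward it.
; A delay timer separates click-to-pick, click-to-place from drag-and-drop.
; Dropping snaps to the last focused square, sending an eligible occupant to the origin square.
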(event `self.ReceiveTick`
  (params (DeltaSeconds :type "Float (single-precision)"))
  (`parent.ReceiveTick` DeltaSeconds)
  (`self.FindFocusedSquare`)
  (`self.UpdateMovingUnitLocation`))

(event `Key|LeftMouseButton`
  (params (Key :type "Key Structure"))
  (:`Pressed`
    (if (not (`self.bMovingUnit`))
      (`/Engine/EditorBlueprintResources/StandardMacros.IsValid` (`self.GetFocusedSquare`)
        (:`Is Valid`
          (`self.IsThereAnyUnitFocusedInSquare`
            (:`Valid`
              (`self.StartMovingUnits`)
              (bind _returnvalue (`KismetSystemLibrary.K2_SetTimerDelegate` (`|CreateDelegate` :!event `StartDragging`) (`self.DragTriggerDelay`)))
              (set `self.DraggingTimer` _returnvalue))))
        (:`Is Not Valid`
          (if (not (`self.bDragging`)) :!label _label
            (`self.StopMovingUnits`))))
      (else
        (goto _label))))
  (:`Released`
    (if (`self.bDragging`)
      (`self.StopDragging`)
      (else
        (`KismetSystemLibrary.K2_ClearAndInvalidateTimerHandle` (`self.DraggingTimer`))))))

(event `FinalStopMove`
  (`KismetSystemLibrary.MoveComponentTo` (`Actor.RootComponent` (`self.MovingUnit`)) (+ (`self.K2_GetActorLocation` (`self.LastFocusedSquare`)) (0.0 0.0 60.0)) (struct) true false 0.02)
  (`/Engine/EditorBlueprintResources/StandardMacros.IsValid` (`self.GetFocusedSquare`)
    (:`Is Valid`
      _)
    (:`Is Not Valid`
      (`/Game/Blueprint/Units/BP_Units.SetFocused` (`self.MovingUnit`) false)))
  (set `self.MovingUnit` null)
  (set `self.bMovingUnit` false))

(fn `FindClosesSquare`
  (`KismetSystemLibrary.LineTraceSingle` (`self.Cursor Location`) (0.0 0.0 0.0) "TraceTypeQuery4"))

(fn `FindFocusedSquare`
  (bind _output_get (set `self.Cursor Location` (`.Location` (`GameplayStatics.BreakHitResult` (`self.GetHitResultUnderCursorByChannel` "TraceTypeQuery3")))))
  (bind _outhits (`KismetSystemLibrary.SphereTraceMulti` _output_get (+ _output_get (0.0 0.0 1.0)) 5.0 "TraceTypeQuery4"))
  (if (> (`KismetArrayLibrary.Array_Length` _outhits) 0)
    (bind (_bblockinghit _binitialoverlap _time _distance _location _impactpoint _normal _impactnormal _physmat _hitactor) (`GameplayStatics.BreakHitResult` (`|GetArrayItem` _outhits)))
    (`/Engine/EditorBlueprintResources/StandardMacros.IsValid` _hitactor
      (:`Is Valid`
        (bind _asbp_square (cast `/Game/Blueprint/Level/BP_Square` _hitactor)
          (:`then`
            (if (!= _asbp_square (`self.FocusedSquare`))
              (`self.UnfocusSquare`)
              (`self.SetFocusedSquare` _asbp_square)))
          (:`CastFailed`
            (`self.UnfocusSquare` :!label _label))))
      (:`Is Not Valid`
        (goto _label)))))

(fn `GetFocusedSquare`
  (returns (ReturnValue :type "/Game/Blueprint/Level/BP_Square Object Reference"))
  (return (`self.FocusedSquare`)))

(fn `GetMovingUnit`
  (returns (ReturnValue :type "/Game/Blueprint/Units/BP_Units Object Reference"))
  (return (`self.MovingUnit`)))

(fn `GetUnitInSquare`
  (returns (ReturnValue :type "/Game/Blueprint/Units/BP_Units Object Reference"))
  (return (`/Game/Blueprint/Level/BP_Square.HostedUnit` (`self.GetFocusedSquare`))))

(fn `ReverseUnitPosition`
  (params (ForUnit :type "/Game/Blueprint/Units/BP_Units Object Reference") (InSquare :type "/Game/Blueprint/Level/BP_Square Object Reference"))
  (`self.K2_SetActorLocation` ForUnit (+ (`self.K2_GetActorLocation` InSquare) (0.0 0.0 60.0)) false true)
  (set `/Game/Blueprint/Level/BP_Square.HostedUnit` ForUnit InSquare))

(fn `SetFocusedSquare`
  (params (Square :type "/Game/Blueprint/Level/BP_Square Object Reference"))
  (set `self.FocusedSquare` Square)
  (if (not (`self.bMovingUnit`))
    (`self.IsThereAnyUnitFocusedInSquare`
      (:`Valid`
        (`/Game/Blueprint/Units/BP_Units.SetFocused` (`self.GetUnitInSquare`) true)))))

(fn `StartDragging`
  (set `self.bDragging` true))

(fn `StartMovingUnits`
  (bind _returnvalue (`self.GetFocusedSquare`))
  (set `self.MovingUnit` (`self.GetUnitInSquare`))
  (set `self.bMovingUnit` true)
  (`/Game/Blueprint/Units/BP_Units.SetDragState` (`self.GetMovingUnit`) true)
  (set `self.InitialMovingSquare` _returnvalue)
  (set `/Game/Blueprint/Level/BP_Square.HostedUnit` null _returnvalue))

(fn `StopDragging`
  (`self.StopMovingUnits`)
  (set `self.bMovingUnit` false))

(fn `StopMovingUnits`
  (bind _returnvalue (`self.GetMovingUnit`))
  (bind _returnvalue_2 (`self.GetFocusedSquare`))
  (`/Engine/EditorBlueprintResources/StandardMacros.IsValid` _returnvalue_2
    (:`Is Valid`
      (set `self.LastFocusedSquare` _returnvalue_2)
      (`self.IsThereAnyUnitFocusedInSquare`
        (:`Valid`
          (`self.ReverseUnitPosition` (`self.GetUnitInSquare`) (`self.InitialMovingSquare`)))
        (:`InValid`
          _)))
    (:`Is Not Valid`
      _))
  (`/Engine/EditorBlueprintResources/StandardMacros.IsValid` _returnvalue
    (:`Is Valid`
      (`/Game/Blueprint/Units/BP_Units.SetDragState` _returnvalue false)
      (set `/Game/Blueprint/Level/BP_Square.HostedUnit` (`self.GetMovingUnit`) (`self.LastFocusedSquare`))
      (`self.FinalStopMove`))))

(fn `UnfocusSquare`
  (bind _focusedsquare (`self.FocusedSquare`))
  (`/Engine/EditorBlueprintResources/StandardMacros.IsValid` (`self.GetFocusedSquare`)
    (:`Is Valid`
      (if (not (`self.bMovingUnit`))
        (`self.IsThereAnyUnitFocusedInSquare`
          (:`Valid`
            (`/Game/Blueprint/Units/BP_Units.SetFocused` (`self.GetUnitInSquare`) false))
          (:`InValid`
            _))))
    (:`Is Not Valid`
      _))
  (`/Engine/EditorBlueprintResources/StandardMacros.IsValid` _focusedsquare
    (:`Is Valid`
      (set `self.LastFocusedSquare` _focusedsquare))
    (:`Is Not Valid`
      _))
  (set `self.FocusedSquare` null))

(fn `UpdateMovingUnitLocation`
  (locals (SquareTempLock :type "Vector Structure" :default (0.0 0.0 0.0)))
  (bind _returnvalue (`self.GetFocusedSquare`))
  (bind _returnvalue_2 (`self.GetMovingUnit`))
  (bind _cursor_location (`self.Cursor Location`))
  (bind _returnvalue_3 (`self.K2_GetActorLocation` _returnvalue_2))
  (bind _returnvalue_4 (`KismetMathLibrary.VInterpTo` _returnvalue_3 (`KismetMathLibrary.MakeVector` (.x (select `bool` true :`false` _cursor_location :`true` (`local.SquareTempLock`))) (.y (select `bool` true :`false` _cursor_location :`true` (`local.SquareTempLock`))) (.z _returnvalue_3)) (`GameplayStatics.GetWorldDeltaSeconds`) (`self.MoveSpeed`)))
  (`/Engine/EditorBlueprintResources/StandardMacros.IsValid` _returnvalue
    (:`Is Valid`
      (set `local.SquareTempLock` (`self.K2_GetActorLocation` _returnvalue)))
    (:`Is Not Valid`
      (set `local.SquareTempLock` _cursor_location)))
  (if (`self.bMovingUnit`)
    (`self.K2_SetActorLocation` _returnvalue_2 _returnvalue_4 false false)
    (`KismetSystemLibrary.DrawDebugArrow` _returnvalue_4 (+ _returnvalue_4 (0.0 0.0 150.0)) 1.0 (struct :`R` 1.0 :`G` 1.0 :`B` 1.0 :`A` 0.483) 0.0 1.0)))

(fn `UserConstructionScript`
  (`parent.UserConstructionScript`))