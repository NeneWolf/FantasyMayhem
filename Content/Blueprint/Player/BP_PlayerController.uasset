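; BP_PlayerController is a player controller that can create the main HUD and run a resolution console command.
; CreateMainHUD, for the local controller only, creates a MainHUD widget, adds it to the player screen and switches input to Game and UI focused on it.
; Nothing in this graph calls CreateMainHUD, and its return node is unconnected.
; Pressing P executes a "r_selfRes 1920x1080" console command.
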(event `Key|P`
  (params (Key :type "Key Structure"))
  (:`Pressed`
    (`KismetSystemLibrary.ExecuteConsoleCommand` "r_selfRes 1920x1080" null)))

(event `self.ReceiveBeginPlay`)

(fn `CreateMainHUD`
  (returns (CreatedWidget :type "UserWidget Object Reference"))
  (if (`self.IsLocalController`)
    (bind _returnvalue (`|CreateWidget` (`self.MainHUD`) self))
    (`UserWidget.AddToPlayerScreen` _returnvalue 0)
    (`WidgetBlueprintLibrary.SetInputMode_GameAndUIEx` self _returnvalue "DoNotLock" false)))

(fn `UserConstructionScript`)