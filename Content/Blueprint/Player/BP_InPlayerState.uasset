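; BP_InPlayerState is a player state Blueprint that provides access to the player's fight zone.
; GetPlayerFightZone returns a cached FightZoneRef, resolving it lazily when invalid by scanning all BP_Battlefield actors for an ID of -1 and taking that battlefield's FightZoneRef01.
; The event graph holds only disabled default events, and the construction script just calls its parent.
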(fn `GetPlayerFightZone`
  (returns (ReturnValue :type "/Game/Blueprint/Level/BP_FightZone Object Reference"))
  (`/Engine/EditorBlueprintResources/StandardMacros.IsValid` (`self.FightZoneRef`)
    (:`Is Valid`
      _)
    (:`Is Not Valid`
      (bind _outactors (`GameplayStatics.GetAllActorsOfClass` "/Game/Blueprint/Level/BP_BattleField.BP_Battlefield_C"))
      (for _array_element _outactors
        (if (== (`/Game/Blueprint/Level/BP_BattleField.ID` _array_element) -1)
          (set `self.FightZoneRef` (`/Game/Blueprint/Level/BP_BattleField.FightZoneRef_01` _array_element))))))
  (return (`self.FightZoneRef`)))

(fn `UserConstructionScript`
  (`parent.UserConstructionScript`))