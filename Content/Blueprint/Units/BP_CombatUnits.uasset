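; Base-style combat unit for networked, AI-driven battles, handling attacks, health, death and revival.
; Tick smoothly rotates it toward its velocity, or toward its target while a rotate flag is set.
; Attacks multicast a data-row montage and damage the target after a short delay; health's RepNotify broadcasts updates and triggers death, which hides the unit and disables collision.
; State changes are authority-only, but always write 0 to the Blackboard; SetTarget and health setup are unfinished.
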(event `self.ReceiveTick`
  (params (DeltaSeconds :type "Float (single-precision)"))
  (`parent.ReceiveTick` DeltaSeconds)
  (`self.RotateTowardsMovementNew`)
  (`self.RotateToTargetNew`))

(event `Multicast_TriggerAttack`
  (`|PlayMontage` (`self.SkeletalMesh`) (`.AttackMontage_21_950658EF4430176EAECC8D95F34A0FCE` (break `/Game/Blueprint/Units/Utility/F_Units` (`self.UnitDataRow`)))))

(event `TriggerAttack`
  (`|ExecutionSequence`
    (:`then_0`
      (`self.Multicast_TriggerAttack`))
    (:`then_1`
      (`KismetSystemLibrary.Delay` 0.3)
      (`self.OnTakeDamageNew` (`self.Target`) (`.Damage_27_F13250CF47A31EB216B17893967BD3A5` (break `/Game/Blueprint/Units/Utility/F_Units` (`self.UnitDataRow`)))))))

(fn `OnDeathNew`
  (`self.Dispatch_OnDeathNew` self)
  (`self.setAIStateNew` "NewEnumerator3")
  (`SceneComponent.SetVisibility` (`self.Capsule`) false true)
  (`self.SetActorEnableCollision` false))

(fn `OnRep_CurrentHealthNew`
  (`self.Dispatch_OnHealthUpdate` self (`self.CurrentHealthNew`))
  (if (== (`self.CurrentHealthNew`) 0.0)
    (`self.OnDeathNew`)))

(fn `OnTakeDamageNew`
  (params (DamageAmount :type "Float (double-precision)"))
  (set `self.CurrentHealthNew` (`KismetMathLibrary.FClamp` (- (`self.CurrentHealthNew`) DamageAmount) 0.0 (`self.MaxHealthNew`))))

(fn `ReviveNew`
  (`self.setAIStateNew` "NewEnumerator0")
  (`SceneComponent.SetVisibility` (`self.Capsule`) true true)
  (`self.SetActorEnableCollision` true)
  (set `self.CurrentHealthNew` (`self.MaxHealthNew`)))

(fn `RotateToTargetNew`
  (bind _returnvalue (`KismetMathLibrary.MakeRotator` 0.0 0.0 (.yaw (`self.K2_GetActorRotation`))))
  (bind _returnvalue_2 (`KismetMathLibrary.MakeRotator` 0.0 0.0 (.yaw (`KismetMathLibrary.FindLookAtRotation` (`self.K2_GetActorLocation`) (`self.K2_GetActorLocation` (`self.Target`))))))
  (if (`self.bShouldRotateNew`)
    (`self.K2_SetActorRotation` (`KismetMathLibrary.RInterpTo` _returnvalue _returnvalue_2 (`GameplayStatics.GetWorldDeltaSeconds`) (`self.RotationSpeedNew`)))
    (if (== _returnvalue _returnvalue_2 :`ErrorTolerance` 2.0)
      (set `self.bShouldRotateNew` false))))

(fn `RotateTowardsMovementNew`
  (bind _returnvalue (`self.GetVelocity`))
  (bind _returnvalue_2 (`self.K2_GetActorLocation`))
  (if (not (`self.bShouldRotateNew`))
    (if (> (`KismetMathLibrary.VSize` _returnvalue) 0.0)
      (`self.K2_SetActorRotation` (`KismetMathLibrary.RInterpTo` (`self.K2_GetActorRotation`) (`KismetMathLibrary.FindLookAtRotation` _returnvalue_2 (+ (* _returnvalue 100.0) _returnvalue_2)) (`GameplayStatics.GetWorldDeltaSeconds`) (`self.RotationSpeedNew`))))))

(fn `setAIStateNew`
  (params (AIState :type "/Game/Blueprint/AI/Utility/EUnitState Enum" :default "NewEnumerator0"))
  (`/Engine/EditorBlueprintResources/ActorMacros.Switch Has Authority`
    (:`Authority`
      (set `self.AIStateNew` AIState)
      (`BlackboardComponent.SetValueAsEnum` (`AIBlueprintHelperLibrary.GetBlackboard` (`self.GetController`)) "State" 0))))

(fn `setCombatMetrics`
  (bind _output_get (set `self.MaxHealthNew` 0.0))
  (set `self.CurrentHealthNew` _output_get))

(fn `SetTarget`
  (`/Engine/EditorBlueprintResources/ActorMacros.Switch Has Authority`))

(fn `StartCombatNew`
  (`self.setAIStateNew` "NewEnumerator1"))

(fn `UserConstructionScript`
  (`parent.UserConstructionScript`))