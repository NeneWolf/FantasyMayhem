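; Base battle unit for a square-grid drag-and-drop combat game, configured from a DT_Units row.
; It snaps onto and registers with the BP_Square found by sphere trace, with custom-depth focus highlighting and a lifted drag pose.
; AI state feeds the blackboard, the battlefield supplies the closest enemy, and attacks multicast a montage before delayed damage.
; Damage updates the widget health bar; death dispatches and hides the unit for later revival.
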(event `self.ReceiveBeginPlay`
  (bind _skeletalmesh (`self.SkeletalMesh`))
  (`self.FindSquare`)
  (`/Game/Blueprint/Units/Widget/WGT_HealthBar.SetMaxHealth` (`self.GetHealthBar`) (`.Health_25_7E8BDCEC4055A5A1BE22D9AD8BF53235` (break `/Game/Blueprint/Units/Utility/F_Units` (`self.UnitDataRow`))))
  (bind _returnvalue (`|SpawnActorFromClass` "/Game/Goblin/StickBP.StickBP_C" (`SceneComponent.GetSocketTransform` _skeletalmesh "weaponstick" "RTS_World") "Undefined" "OverrideRootScale" null null))
  (`self.K2_AttachToComponent` _returnvalue _skeletalmesh "weaponstick" "SnapToTarget" "SnapToTarget" "SnapToTarget" true))

(event `self.ReceiveTick`
  (params (DeltaSeconds :type "Float (single-precision)"))
  (`self.RotateTowardsMovement`)
  (`self.RotateToTarget`))

(event `Multicast_TriggerAttack`
  (`|PlayMontage` (`self.SkeletalMesh`) (`.AttackMontage_22_AC2727624E5AE93CA480C8B3F7DEA7CF` (break `/Game/Blueprint/Units/Utility/F_Units` (`self.UnitDataRow`)))))

(event `TriggerAttack`
  (`|ExecutionSequence`
    (:`then_0`
      (`self.Multicast_TriggerAttack`))
    (:`then_1`
      (`KismetSystemLibrary.Delay` 0.3)
      (`self.OnTakeDamage` (`self.AttackTarget`) (`.Damage_30_9B277C214868EEAE497927A9ED498F3B` (break `/Game/Blueprint/Units/Utility/F_Units` (`self.UnitDataRow`)))))))

(fn `ExtractDataFromRow`
  (bind _skeletalmesh (`self.SkeletalMesh`))
  (bind _returnvalue (`|GetDataTableRow` "/Game/Blueprint/Data/DT_Units.DT_Units" (`.RowName` (break `DataTableRowHandle` (`self.UnitRow`))))
    (:`then`
      (bind _output_get (set `self.UnitDataRow` _returnvalue))
      (bind ((`Skeletal_10_253F8363405F346D0C52D799A356434C` _skeletal) (`AnimInstance_18_9C1AB54145DBE62C5B79F6A542748F32` _animinstance) (`Health_25_7E8BDCEC4055A5A1BE22D9AD8BF53235` _health)) (break `/Game/Blueprint/Units/Utility/F_Units` _output_get))
      (`SkinnedMeshComponent.SetSkinnedAssetAndUpdate` _skeletalmesh _skeletal true)
      (`SkeletalMeshComponent.SetAnimInstanceClass` _skeletalmesh _animinstance)
      (bind _output_get_2 (set `self.MaxHealth` _health))
      (set `self.CurrentHealth` _output_get_2))))

(fn `FindSquare`
  (bind _returnvalue (`self.K2_GetActorLocation`))
  (bind _initialsquare (`self.InitialSquare`))
  (`/Engine/EditorBlueprintResources/StandardMacros.IsValid` _initialsquare
    (:`Is Valid`
      (set `/Game/Blueprint/Level/BP_Square.HostedUnit` null _initialsquare))
    (:`Is Not Valid`
      _))
  (bind _outhits (`KismetSystemLibrary.SphereTraceMulti` _returnvalue (+ _returnvalue (0.0 0.0 1.0)) 5.0 "TraceTypeQuery4"))
  (for _array_element _outhits
    (bind (_bblockinghit _binitialoverlap _time _distance _location _impactpoint _normal _impactnormal _physmat _hitactor) (`GameplayStatics.BreakHitResult` _array_element))
    (if (== (`GameplayStatics.GetObjectClass` _hitactor) "/Game/Blueprint/Level/BP_Square.BP_Square_C")
      (bind _asbp_square (cast `/Game/Blueprint/Level/BP_Square` _hitactor))
      (set `/Game/Blueprint/Level/BP_Square.HostedUnit` self _asbp_square)
      (`self.K2_SetActorLocation` (+ (`self.K2_GetActorLocation` _asbp_square) (0.0 0.0 60.0)))
      (set `self.InitialSquare` _asbp_square))))

(fn `GetHealthBar`
  (returns (ReturnValue :type "/Game/Blueprint/Units/Widget/WGT_HealthBar Object Reference"))
  (`/Engine/EditorBlueprintResources/StandardMacros.IsValid` (`self.HealthBarRef`)
    (:`Is Valid`
      _)
    (:`Is Not Valid`
      (bind _aswgt_health_bar (cast `/Game/Blueprint/Units/Widget/WGT_HealthBar` (`WidgetComponent.GetUserWidgetObject` (`self.WGC_HealthBar`))))
      (set `self.HealthBarRef` _aswgt_health_bar)))
  (return (`self.HealthBarRef`)))

(fn `OnDeath`
  (`self.Dispatch_OnDeath` self)
  (`self.SetAIState` "NewEnumerator3")
  (`SceneComponent.SetVisibility` (`self.Capsule`) false true)
  (`self.SetActorEnableCollision` false))

(fn `OnTakeDamage`
  (params (Amount :type "Float (double-precision)"))
  (set `self.CurrentHealth` (`KismetMathLibrary.FClamp` (- (`self.CurrentHealth`) Amount) 0.0 (`self.MaxHealth`)))
  (`/Game/Blueprint/Units/Widget/WGT_HealthBar.SetCurrentHealth` (`self.GetHealthBar`) (`self.CurrentHealth`))
  (if (== (`self.CurrentHealth`) 0.0)
    (`self.OnDeath`)))

(fn `ReviveUnit`
  (`self.SetAIState` "NewEnumerator0")
  (`SceneComponent.SetVisibility` (`self.Capsule`) true true)
  (`self.SetActorEnableCollision` true)
  (set `self.CurrentHealth` (`self.MaxHealth`)))

(fn `RotateToTarget`
  (bind _returnvalue (`KismetMathLibrary.MakeRotator` 0.0 0.0 (.yaw (`self.K2_GetActorRotation`))))
  (bind _returnvalue_2 (`KismetMathLibrary.MakeRotator` 0.0 0.0 (.yaw (`KismetMathLibrary.FindLookAtRotation` (`self.K2_GetActorLocation`) (`self.K2_GetActorLocation` (`self.AttackTarget`))))))
  (if (`self.bShouldRotate`)
    (`self.K2_SetActorRotation` (`KismetMathLibrary.RInterpTo` _returnvalue _returnvalue_2 (`GameplayStatics.GetWorldDeltaSeconds`) (`self.RotationSpeed`)))
    (if (== _returnvalue _returnvalue_2 :`ErrorTolerance` 1.0)
      (set `self.bShouldRotate` false))))

(fn `RotateTowardsMovement`
  (bind _returnvalue (`self.GetVelocity`))
  (bind _returnvalue_2 (`self.K2_GetActorLocation`))
  (if (> (`KismetMathLibrary.VSize` _returnvalue) 0.0)
    (`self.K2_SetActorRotation` (`KismetMathLibrary.RInterpTo` (`self.K2_GetActorRotation`) (`KismetMathLibrary.FindLookAtRotation` _returnvalue_2 (+ (* _returnvalue 100.0) _returnvalue_2)) (`GameplayStatics.GetWorldDeltaSeconds`) (`self.RotationSpeed`)))))

(fn `SetAIState`
  (params (NewState :type "/Game/Blueprint/AI/Utility/EUnitState Enum" :default "NewEnumerator0"))
  (set `self.AIState` NewState)
  (`BlackboardComponent.SetValueAsEnum` (`AIBlueprintHelperLibrary.GetBlackboard` (`self.GetController`)) "State" NewState))

(fn `SetAttackedTarget`
  (returns (ChosenTarget :type "/Game/Blueprint/Units/BP_Units Object Reference"))
  (bind _returnvalue (`/Game/Blueprint/Level/BP_BattleField.GetClosestEnemyUnit` (`self.CurrentBattlefield`) self))
  (`/Engine/EditorBlueprintResources/StandardMacros.IsValid` _returnvalue
    (:`Is Valid`
      (set `self.AttackTarget` _returnvalue)
      (return (`self.AttackTarget`)))
    (:`Is Not Valid`
      (`self.SetAIState` "NewEnumerator0")
      (return null))))

(fn `SetDragState`
  (params (Enable :type Boolean))
  (bind _skeletalmesh (`self.SkeletalMesh`))
  (`self.SetMeshRelativeState` Enable)
  (if Enable
    (`SceneComponent.K2_SetRelativeRotation` _skeletalmesh (struct :`Roll` 25.0) false false)
    (else
      (`SceneComponent.K2_SetRelativeRotation` _skeletalmesh (struct :`Yaw` -90.0) false false))))

(fn `SetFocused`
  (params (bFocused :type Boolean))
  (bind _skeletalmesh (`self.SkeletalMesh`))
  (if bFocused
    (`PrimitiveComponent.SetRenderCustomDepth` _skeletalmesh true)
    (`PrimitiveComponent.SetCustomDepthStencilValue` _skeletalmesh 249)
    (else
      (`PrimitiveComponent.SetRenderCustomDepth` _skeletalmesh false))))

(fn `SetMeshRelativeState`
  (params (Dragged :type Boolean))
  (bind _skeletalmesh (`self.SkeletalMesh`))
  (bind _returnvalue (`SkeletalMeshComponent.GetAnimInstance` _skeletalmesh))
  (if Dragged
    (`SceneComponent.K2_SetRelativeLocation` _skeletalmesh (`KismetMathLibrary.MakeVector` 0.0 0.0 120.0) false false)
    (message `/Game/Blueprint/Units/Utility/BPI_AnimCommunication.SetDraggedAnimState` _returnvalue true)
    (else
      (`SceneComponent.K2_SetRelativeLocation` (`self.SkeletalMesh`) (`KismetMathLibrary.MakeVector` 0.0 0.0 -60.0) false false)
      (message `/Game/Blueprint/Units/Utility/BPI_AnimCommunication.SetDraggedAnimState` _returnvalue false))))

(fn `StartCombat`
  (`self.SetAIState` "NewEnumerator1"))

(fn `UserConstructionScript`
  (`self.ExtractDataFromRow`)
  (`self.FindSquare`))