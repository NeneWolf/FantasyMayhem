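; BP_BattleField runs auto-battler style fights between teams of units placed on board squares, then returns to the recruit phase.
; StartCombat registers hosted units by team, saves their pre-combat positions, binds death events and starts their combat.
; Deaths shrink team lists; when a team empties and any remain, it prints a winner, then after a delay revives units and restores their positions.
; It also provides a nearest-enemy lookup that skips units in one AI state.
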(event `GoToRecruitPhase`
  (bind _units (`self.Units`))
  (`KismetSystemLibrary.Delay` 3.0)
  (`/Game/Blueprint/Units/BP_Units.ReviveUnit` _units)
  (for _array_element _units
    (`self.K2_SetActorLocation` _array_element (`/Game/Blueprint/Units/BP_Units.PreCombatLocation` _array_element) false true)
    (`self.K2_SetActorRotation` _array_element (struct :`Yaw` 180.0) true)))

(fn `FindUnitsInBattlefield`
  (locals (tempUnitArray :type "Array of /Game/Blueprint/Units/BP_Units Object Reference"))
  (bind _unitsfromteam (`self.UnitsFromTeam`))
  (for _array_element (`self.Squares`)
    (bind _hostedunit (`/Game/Blueprint/Level/BP_Square.HostedUnit` _array_element))
    (`/Engine/EditorBlueprintResources/StandardMacros.IsValid` _hostedunit
      (:`Is Valid`
        (set `/Game/Blueprint/Units/BP_Units.PreCombatLocation` (+ (`self.K2_GetActorLocation` _array_element) (0.0 0.0 60.0)) _hostedunit)
        (set `/Game/Blueprint/Units/BP_Units.CurrentBattlefield` self _hostedunit)
        (bind _team (`/Game/Blueprint/Units/BP_Units.Team` _hostedunit))
        (set `local.tempUnitArray` (`.Units_3_D2C7616D4760A314012DE98DD810B1CA` (break `/Game/Blueprint/Units/Utility/FUnits` (`BlueprintMapLibrary.Map_Find` _unitsfromteam _team))))
        (`KismetArrayLibrary.Array_Append` (`local.tempUnitArray`) (`|MakeArray` _hostedunit))
        (`BlueprintMapLibrary.Map_Add` _unitsfromteam _team (make `/Game/Blueprint/Units/Utility/FUnits` (`local.tempUnitArray`)))
        (add `/Game/Blueprint/Units/BP_Units.Dispatch_OnDeath` _hostedunit (`|CreateDelegate` :!event `OnUnitDeath`))))))

(fn `GetClosestEnemyUnit`
  (params (InUnit :type "/Game/Blueprint/Units/BP_Units Object Reference"))
  (returns (ReturnValue :type "/Game/Blueprint/Units/BP_Units Object Reference"))
  (locals (closestDistance :type "Float (double-precision)" :default 2000000.0) (owningTeam :type Integer :default 0) (tempClosestUnit :type "/Game/Blueprint/Units/BP_Units Object Reference"))
  (set `local.owningTeam` (`/Game/Blueprint/Units/BP_Units.Team` InUnit))
  (for _array_element (`self.Units`)
    (if (`|EnumInequality` (`/Game/Blueprint/Units/BP_Units.AIState` _array_element) "NewEnumerator3")
      (if (!= (`/Game/Blueprint/Units/BP_Units.Team` _array_element) (`local.owningTeam`))
        (bind _returnvalue (`self.GetDistanceTo` _array_element (`local.InUnit`)))
        (if (<= _returnvalue (`local.closestDistance`))
          (set `local.closestDistance` _returnvalue)
          (set `local.tempClosestUnit` _array_element)))))
  (return (`local.tempClosestUnit`)))

(fn `IsTeamEmpty`
  (params (teamID :type Integer))
  (returns (ReturnValue :type Boolean))
  (return (== (`KismetArrayLibrary.Array_Length` (`.Units_3_D2C7616D4760A314012DE98DD810B1CA` (break `/Game/Blueprint/Units/Utility/FUnits` (`BlueprintMapLibrary.Map_Find` (`self.UnitsFromTeam`) teamID)))) 0)))

(fn `OnUnitDeath`
  (params (InUnit :type "/Game/Blueprint/Units/BP_Units Object Reference"))
  (bind _team (`/Game/Blueprint/Units/BP_Units.Team` InUnit))
  (bind _fightingteams (`self.FightingTeams`))
  (`self.RemoveUnitFromTeam` InUnit)
  (if (`self.IsTeamEmpty` _team)
    (`KismetArrayLibrary.Array_RemoveItem` _fightingteams _team)
    (if (> (`KismetArrayLibrary.Array_Length` _fightingteams) 0)
      (`KismetSystemLibrary.PrintString` (`KismetStringLibrary.Concat_StrStr` "Winner is: Team " (`KismetStringLibrary.Conv_IntToString` (`|GetArrayItem` (`self.FightingTeams`)))) true true (struct :`G` 1.0 :`A` 1.0) 5.0)
      (set `self.IsBattleOn` false)
      (`self.GoToRecruitPhase`))))

(fn `RemoveUnitFromTeam`
  (params (InUnit :type "/Game/Blueprint/Units/BP_Units Object Reference"))
  (locals (tempUnits :type "Array of /Game/Blueprint/Units/BP_Units Object Reference"))
  (bind (_value _returnvalue) (`BlueprintMapLibrary.Map_Find` (`self.UnitsFromTeam`) (`/Game/Blueprint/Units/BP_Units.Team` InUnit)))
  (if _returnvalue
    (bind _output_get (set `local.tempUnits` (`.Units_3_D2C7616D4760A314012DE98DD810B1CA` (break `/Game/Blueprint/Units/Utility/FUnits` _value))))
    (if (`KismetArrayLibrary.Array_Contains` _output_get InUnit)
      (`KismetArrayLibrary.Array_RemoveItem` (`local.tempUnits`) InUnit)
      (`BlueprintMapLibrary.Map_Add` (`self.UnitsFromTeam`) (`/Game/Blueprint/Units/BP_Units.Team` InUnit) (make `/Game/Blueprint/Units/Utility/FUnits` (`local.tempUnits`))))))

(fn `StartCombat`
  (set `self.IsBattleOn` true)
  (`self.FindUnitsInBattlefield`)
  (`self.FindUnitsInGrid`)
  (`/Game/Blueprint/Units/BP_Units.StartCombat` (`self.Units`)))

(fn `UserConstructionScript`
  (`parent.UserConstructionScript`))