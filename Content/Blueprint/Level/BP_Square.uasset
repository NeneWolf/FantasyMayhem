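; BP_Square is a square level tile with a HostedUnit reference, which starts cleared.
; Its construction script calls UpdateRelativeLocation, which scales a thin StaticMesh slab and a Box component from the Size variable.
; Both are then raised by half their height, intended to rest them on the actor's origin instead of centering them on it.
; The Blueprint has no active runtime event logic.
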(fn `UpdateRelativeLocation`
  (bind _box (`self.Box`))
  (bind _staticmesh (`self.StaticMesh`))
  (bind _returnvalue (/ (`self.Size`) 100.0))
  (bind _returnvalue_2 (* (1.0 1.0 1.0) _returnvalue))
  (`SceneComponent.SetWorldScale3D` _staticmesh (`KismetMathLibrary.MakeVector` (.x _returnvalue_2) (.y _returnvalue_2) 0.01))
  (`SceneComponent.SetRelativeScale3D` (`self.Box`) _returnvalue_2)
  (`SceneComponent.K2_SetRelativeLocation` _staticmesh (`KismetMathLibrary.MakeVector` 0.0 0.0 (* (.z (/ (`SceneComponent.RelativeScale3D` _staticmesh) 2.0)) 100.0)) false false)
  (`SceneComponent.K2_SetRelativeLocation` _box (`KismetMathLibrary.MakeVector` 0.0 0.0 (* (.z (`BoxComponent.BoxExtent` _box)) _returnvalue)) false false))

(fn `UserConstructionScript`
  (`self.UpdateRelativeLocation`)
  (set `self.HostedUnit` null))