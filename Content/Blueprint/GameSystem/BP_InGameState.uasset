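; BP_InGameState is the match state that alternates the game between Recruit and Combat phases, starting in Recruit on BeginPlay.
; Each phase change updates CurrentPhase, fires a new-phase dispatcher and starts a one-shot timer, whose end handler flips phases.
; Recruit calls player matching, shop refresh and income; Combat awaits combat data on authority only.
; These gameplay steps and the battlefield lookup are still empty stubs.
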(event `self.ReceiveBeginPlay`
  (`parent.ReceiveBeginPlay`)
  (`self.GoToPhase` "NewEnumerator1"))

(fn `AwaitCombatData`)

(fn `GenerateIncome`)

(fn `GetPlayerBattlefield`
  (params (InPlayer :type String))
  (returns (ReturnValue :type Integer))
  (return 0))

(fn `GoToCombatPhase`
  (`self.SetPhase` "NewEnumerator2")
  (`self.LaunchPhaseTimer` (`self.MaxCombatPhaseDuration`))
  (`/Engine/EditorBlueprintResources/ActorMacros.Switch Has Authority`
    (:`Authority`
      (`self.AwaitCombatData`))))

(fn `GoToPhase`
  (params (InNewPhase :type "/Game/Blueprint/GameSystem/Utility/EGamePhase Enum" :default "NewEnumerator0"))
  (switch `/Game/Blueprint/GameSystem/Utility/EGamePhase` InNewPhase
    (:`NewEnumerator1`
      (`self.GoToRecruitPhase`))
    (:`NewEnumerator2`
      (`self.GoToCombatPhase`))))

(fn `GoToRecruitPhase`
  (`self.SetPhase` "NewEnumerator1")
  (`self.MatchPlayers`)
  (`self.RefreshPlayerShops`)
  (`self.GenerateIncome`)
  (`self.LaunchPhaseTimer` (`self.RecruitPhaseDuration`)))

(fn `LaunchPhaseTimer`
  (params (TimerDuration :type "Float (double-precision)"))
  (bind _returnvalue (`KismetSystemLibrary.K2_SetTimerDelegate` (`|CreateDelegate` :!event `OnPhaseTimerEnd`) TimerDuration))
  (set `self.PhaseTimer` _returnvalue))

(fn `MatchPlayers`)

(fn `OnPhaseTimerEnd`
  (switch `/Game/Blueprint/GameSystem/Utility/EGamePhase` (`self.CurrentPhase`)
    (:`NewEnumerator1`
      (`self.GoToPhase` "NewEnumerator2"))
    (:`NewEnumerator2`
      (`self.GoToPhase` "NewEnumerator1"))))

(fn `RefreshPlayerShops`)

(fn `SetPhase`
  (params (NewPhase :type "/Game/Blueprint/GameSystem/Utility/EGamePhase Enum" :default "NewEnumerator0"))
  (bind _output_get (set `self.CurrentPhase` NewPhase))
  (`self.Dispatch_OnNewPhaseStarted` _output_get))

(fn `UserConstructionScript`
  (`parent.UserConstructionScript`))