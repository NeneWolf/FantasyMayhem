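; BP_Ent is a tree-creature Blueprint that carries a waterball on its skeletal mesh.
; The construction script makes the separate leaves mesh follow the main mesh's pose through Master Pose Component and sets its visibility from the LeavesVisability variable.
; On BeginPlay it spawns a BP_waterball actor at the "waterball" socket and snaps it to that socket.
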(event `self.ReceiveBeginPlay`
  (bind _returnvalue (`|SpawnActorFromClass` "/Game/qinpack/greenent/BP_waterball.BP_waterball_C" (`SceneComponent.GetSocketTransform` (`self.Mesh`) "waterball" "RTS_World") "Undefined" "OverrideRootScale" null null))
  (`self.K2_AttachToComponent` _returnvalue (`self.Mesh`) "waterball" "SnapToTarget" "SnapToTarget" "SnapToTarget" true))

(fn `UserConstructionScript`
  (`SkinnedMeshComponent.SetLeaderPoseComponent` (`self.SK_Ent_Leaves`) (`self.Mesh`) true)
  (`SceneComponent.SetVisibility` (`self.SK_Ent_Leaves`) (`self.Leaves Visability`) false))